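; Player pawn acting as a top-down camera, with key-axis and screen-edge panning plus a hold-to-double speed boost.
; Middle mouse opens a per-tick gate that yaws PlayerBase and pitches the SpringArm within limits, suspending edge scroll.
; Scroll zoom changes clamped arm length, with optional invert and zoom-to-cursor that moves the pawn to the deprojected mouse point.
; A timeline eases rotation and zoom back on ResetCamera, and middle mouse interrupts it.
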(event `self.ReceiveBeginPlay`
  (`|ExecutionSequence`
    (:`then_0`
      (bind _asplayer_controller (cast `PlayerController` (`self.GetController`)))
      (set `self.PlayerController` _asplayer_controller)
      (set `self.DefaultMovementSpeed` (`self.MovementSpeed`)))
    (:`then_1`
      (`/Engine/EditorBlueprintResources/StandardMacros.IsValid` (`self.PlayerController`)
        (:`Is Valid`
          (`|ExecutionSequence`
            (:`then_0`
              (set `PlayerController.bShowMouseCursor` true (`self.PlayerController`)))))))))

(event `self.ReceiveTick`
  (params (DeltaSeconds :type "Float (single-precision)"))
  (`|ExecutionSequence`
    (:`then_0`
      (`self.Tick_MouseRotation`))
    (:`then_1`
      (`self.Tick_MouseMovement`))))

(event `InputAxis|MoveForward`
  (params (AxisValue :type "Float (single-precision)"))
  ;[1 1 1] Movement WASD - Arrows
  (`self.AddForward` AxisValue))

(event `InputAction|IncreaseCameraSpeed`
  (params (Key :type "Key Structure"))
  ;[1 1 1] Mouse Movement
  (:`Pressed`
    (set `self.MovementSpeed` (* (`self.DefaultMovementSpeed`) 2.0)))
  (:`Released`
    (set `self.MovementSpeed` (`self.DefaultMovementSpeed`))))

(event `InputAxis|MoveRight`
  (params (AxisValue :type "Float (single-precision)"))
  ;[1 1 1] Movement WASD - Arrows
  (`self.AddRight` AxisValue))

(event `InputAction|ZoomIn`
  (params (Key :type "Key Structure"))
  (bind _returnvalue (`KismetMathLibrary.SelectFloat` 1.0 -1.0 (`self.bInvertedZoom`)))
  ;[1 1 1] Mouse Scroll Zoom
  (:`Pressed`
    (set `SpringArmComponent.TargetArmLength` (`self.GetNewTargetLength` _returnvalue) (`self.SpringArm`))
    (`self.ZoomToPosition` _returnvalue)))

(event `InputAction|ZoomOut`
  (params (Key :type "Key Structure"))
  (bind _returnvalue (`KismetMathLibrary.SelectFloat` -1.0 1.0 (`self.bInvertedZoom`)))
  ;[1 1 1] Mouse Scroll Zoom
  (:`Pressed`
    (set `SpringArmComponent.TargetArmLength` (`self.GetNewTargetLength` _returnvalue) (`self.SpringArm`))
    (`self.ZoomToPosition` _returnvalue)))

(event `ZoomToPosition`
  (params (Value :type "Float (double-precision)"))
  (bind (_locationx _locationy) (`PlayerController.GetMousePosition` (`self.PlayerController`)))
  (bind (_worldlocation _worlddirection) (`PlayerController.DeprojectMousePositionToWorld` (`self.PlayerController`)))
  (bind _returnvalue (`KismetMathLibrary.MakeVector2D` _locationx _locationy))
  ;[1 1 1] ZoomToPosition
  (if (`self.bZoomToMouse`)
    (if (and (< Value 0.0) (> (`SpringArmComponent.TargetArmLength` (`self.SpringArm`)) (`self.MaximumZoom`)))
      (if (not (not (!= _returnvalue (`self.LastMousePosition`) :`ErrorTolerance` 20.0)))
        (set `self.StartZoomPosition` (`KismetMathLibrary.MakeVector` (.x (+ _worldlocation (* _worlddirection (`SpringArmComponent.TargetArmLength` (`self.SpringArm`))))) (.y (+ _worldlocation (* _worlddirection (`SpringArmComponent.TargetArmLength` (`self.SpringArm`))))))))
      (set `self.LastMousePosition` _returnvalue)
      (`self.K2_SetActorLocation` (`self.StartZoomPosition`)))))

(event `Tick_MouseRotation`
  (bind _playerbase (`self.PlayerBase`))
  (bind (_relativerotation_roll _relativerotation_pitch) (`KismetMathLibrary.BreakRotator` (`SceneComponent.RelativeRotation` (`self.SpringArm`))))
  (bind (_relativerotation_roll_2 _relativerotation_pitch_2 _relativerotation_yaw) (`KismetMathLibrary.BreakRotator` (`SceneComponent.RelativeRotation` _playerbase)))
  ;[1 1 1] Mouse Middle Button Movement
  (`/Engine/EditorBlueprintResources/StandardMacros.Gate` true :!label _label
    (:`Exit`
      (`|ExecutionSequence`
        (:`then_0`
          (`SceneComponent.K2_SetRelativeRotation` _playerbase (`KismetMathLibrary.MakeRotator` 0.0 0.0 (+ _relativerotation_yaw (`self.GetInputAxisKeyValue`))) false false)
          (set `PlayerController.CurrentMouseCursor` "GrabHandClosed" (`self.PlayerController`)))
        (:`then_1`
          (`SceneComponent.K2_SetRelativeRotation` (`self.SpringArm`) (`KismetMathLibrary.MakeRotator` 0.0 (`KismetMathLibrary.FClamp` (+ _relativerotation_pitch (`self.GetInputAxisKeyValue`)) -90.0 -35.0)) false false)
          (set `PlayerController.CurrentMouseCursor` "GrabHandClosed" (`self.PlayerController`)))))))

(event `Key|MiddleMouseButton`
  (params (Key :type "Key Structure"))
  (bind _playerbase (`self.PlayerBase`))
  ;[1 1 1] Mouse Middle Button Movement
  (:`Pressed`
    (set `self.bIsRotatingCamera` true)
    (`|ExecutionSequence`
      (:`then_0`
        (goto _label :!via `Open`))
      (:`then_1`
        (bind (_direction _alpha) (`Timeline|Timeline_ResetCamera` :!via `Stop` :!label _label_2)
          (:`Update`
            (`|ExecutionSequence`
              (:`then_0`
                (`SceneComponent.K2_SetRelativeRotation` _playerbase (`KismetMathLibrary.RLerp` (`SceneComponent.RelativeRotation` _playerbase) (struct) _alpha) false false))
              (:`then_1`
                (set `SpringArmComponent.TargetArmLength` (`KismetMathLibrary.Lerp` (`SpringArmComponent.TargetArmLength` (`self.SpringArm`)) (`self.MinimumZoom`) _alpha) (`self.SpringArm`)))))))))
  (:`Released`
    (set `self.bIsRotatingCamera` false)
    (set `PlayerController.CurrentMouseCursor` "Default" (`self.PlayerController`))
    (goto _label :!via `Close`)))

(event `InputAction|ResetCamera`
  (params (Key :type "Key Structure"))
  ;[1 1 1] Mouse Middle Button Movement
  (:`Pressed`
    (goto _label_2 :!via `PlayFromStart`)))

(event `Tick_MouseMovement`
  (bind _playercontroller (`self.PlayerController`))
  (bind (_sizex _sizey) (`PlayerController.GetViewportSize` _playercontroller))
  (bind (_locationx _locationy _returnvalue) (`PlayerController.GetMousePosition` _playercontroller))
  ;[1 1 1] Side Scrolling
  (if (and (not (`self.bIsRotatingCamera`)) _returnvalue)
    (`|ExecutionSequence`
      (:`then_0`
        (if (< _locationx (`self.EdgeScrollSensitivity`))
          (`self.AddRight` -1.0)
          (elif (> _locationx (- (`KismetMathLibrary.Conv_IntToDouble` _sizex) (`self.EdgeScrollSensitivity`)))
            (`self.AddRight` 1.0))))
      (:`then_1`
        (if (< _locationy (`self.EdgeScrollSensitivity`))
          (`self.AddForward` 1.0)
          (elif (> _locationy (- (`KismetMathLibrary.Conv_IntToDouble` _sizey) (`self.EdgeScrollSensitivity`)))
            (`self.AddForward` -1.0)))))))

(fn `AddForward`
  (params (axis :type "Float (double-precision)"))
  (`self.K2_AddActorWorldOffset` (* (`SceneComponent.GetForwardVector` (`self.PlayerBase`)) (* (`self.MovementSpeed`) axis))))

(fn `AddRight`
  (params (axis :type "Float (double-precision)"))
  (`self.K2_AddActorWorldOffset` (* (`SceneComponent.GetRightVector` (`self.PlayerBase`)) (* axis (`self.MovementSpeed`)))))

(fn `GetNewTargetLength`
  (params (Axis :type "Float (double-precision)"))
  (returns (ReturnValue :type "Float (double-precision)"))
  (return (`KismetMathLibrary.FClamp` (+ (* Axis (`self.ScrollSensitivity`)) (`SpringArmComponent.TargetArmLength` (`self.SpringArm`))) (`self.MaximumZoom`) (`self.MinimumZoom`))))

(fn `UserConstructionScript`)