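; Player camera pawn for a top-down, strategy-style view, with axis-input and screen-edge panning, a speed boost and a visible cursor.
; Movement offsets the actor along PlayerBase's axes per frame, without delta-time scaling.
; A gate on middle mouse drives PlayerBase yaw and clamped SpringArm pitch, suppressing edge scroll.
; Zoom adjusts clamped arm length, optionally jumping toward a cached deprojected cursor point, while a timeline eases camera reset.
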(event `self.ReceiveBeginPlay`
  (`|ExecutionSequence`
    (:`then_0`
      (bind _asplayer_controller (cast `PlayerController` (`self.GetController`)))
      (set `self.PlayerController` _asplayer_controller)
      (set `self.DefaultMovementSpeed` (`self.MovementSpeed`)))
    (:`then_1`
      (`/Engine/EditorBlueprintResources/StandardMacros.IsValid` (`self.PlayerController`)
        (:`Is Valid`
          (`|ExecutionSequence`
            (:`then_0`
              (set `PlayerController.bShowMouseCursor` true (`self.PlayerController`)))))))))

(event `self.ReceiveTick`
  (params (DeltaSeconds :type "Float (single-precision)"))
  (`|ExecutionSequence`
    (:`then_0`
      (`self.Tick_MouseRotation`))
    (:`then_1`
      (`self.Tick_MouseMovement`))))

(event `InputAxis|MoveForward`
  (params (AxisValue :type "Float (single-precision)"))
  ;[1 1 1] Movement WASD - Arrows
  (`self.AddForward` AxisValue))

(event `InputAxis|MoveRight`
  (params (AxisValue :type "Float (single-precision)"))
  ;[1 1 1] Movement WASD - Arrows
  (`self.AddRight` AxisValue))

(event `InputAction|ZoomIn`
  (params (Key :type "Key Structure"))
  (bind _returnvalue (`self.GetInputAxisKeyValue`))
  (bind _playercontroller (`self.PlayerController`))
  (bind (_locationx _locationy) (`PlayerController.GetMousePosition` (`self.PlayerController`)))
  (bind (_locationx_2 _locationy_2) (`PlayerController.GetMousePosition` _playercontroller))
  (bind _returnvalue_2 (`KismetMathLibrary.MakeVector2D` _locationx _locationy))
  (bind (_worldposition _worlddirection) (`GameplayStatics.DeprojectScreenToWorld` _playercontroller (`KismetMathLibrary.MakeVector2D` _locationx_2 _locationy_2)))
  (bind _returnvalue_3 (`KismetMathLibrary.SelectFloat` _returnvalue (* _returnvalue -1.0) (`self.bInvertedZoom`)))
  ;[1 1 1] Mouse Scroll Zoom
  (:`Pressed`
    (set `SpringArmComponent.TargetArmLength` (`KismetMathLibrary.FClamp` (+ (* _returnvalue_3 (`self.ScrollSensitivity`)) (`SpringArmComponent.TargetArmLength` (`self.SpringArm`))) (`self.MaximumZoom`) (`self.MinimumZoom`)) (`self.SpringArm`) :!label _label)
    (if (and (< _returnvalue_3 0.0) (`self.bZoomToMouse`))
      (if (and (not (!= _returnvalue_2 (`self.LastMousePosition`) :`ErrorTolerance` 20.0)) (> (`SpringArmComponent.TargetArmLength` (`self.SpringArm`)) (`self.MaximumZoom`)))
        (set `self.LastMousePosition` _returnvalue_2)
        (`self.K2_SetActorLocation` (`self.StartZoomPosition`) true)
        (else
          (set `self.LastMousePosition` _returnvalue_2)
          (set `self.StartZoomPosition` (`KismetMathLibrary.MakeVector` (.x (+ _worldposition (* _worlddirection (`SpringArmComponent.TargetArmLength` (`self.SpringArm`))))) (.y (+ _worldposition (* _worlddirection (`SpringArmComponent.TargetArmLength` (`self.SpringArm`))))))))))))

(event `InputAction|ZoomOut`
  (params (Key :type "Key Structure"))
  ;[1 1 1] Mouse Scroll Zoom
  (:`Pressed`
    (goto _label)))

(event `Tick_MouseRotation`
  (bind _playerbase (`self.PlayerBase`))
  (bind (_relativerotation_roll _relativerotation_pitch) (`KismetMathLibrary.BreakRotator` (`SceneComponent.RelativeRotation` (`self.SpringArm`))))
  (bind (_relativerotation_roll_2 _relativerotation_pitch_2 _relativerotation_yaw) (`KismetMathLibrary.BreakRotator` (`SceneComponent.RelativeRotation` _playerbase)))
  ;[1 1 1] Mouse Middle Button Movement
  (`/Engine/EditorBlueprintResources/StandardMacros.Gate` true :!label _label_2
    (:`Exit`
      (`|ExecutionSequence`
        (:`then_0`
          (`SceneComponent.K2_SetRelativeRotation` _playerbase (`KismetMathLibrary.MakeRotator` 0.0 0.0 (+ _relativerotation_yaw (`self.GetInputAxisKeyValue`))) false false)
          (set `PlayerController.CurrentMouseCursor` "GrabHandClosed" (`self.PlayerController`)))
        (:`then_1`
          (`SceneComponent.K2_SetRelativeRotation` (`self.SpringArm`) (`KismetMathLibrary.MakeRotator` 0.0 (`KismetMathLibrary.FClamp` (+ _relativerotation_pitch (`self.GetInputAxisKeyValue`)) -90.0 -35.0)) false false)
          (set `PlayerController.CurrentMouseCursor` "GrabHandClosed" (`self.PlayerController`)))))))

(event `Key|MiddleMouseButton`
  (params (Key :type "Key Structure"))
  (bind _playerbase (`self.PlayerBase`))
  ;[1 1 1] Mouse Middle Button Movement
  (:`Pressed`
    (set `self.bIsRotatingCamera` true)
    (`|ExecutionSequence`
      (:`then_0`
        (goto _label_2 :!via `Open`))
      (:`then_1`
        (bind (_direction _alpha) (`Timeline|Timeline_ResetCamera` :!via `Stop` :!label _label_3)
          (:`Update`
            (`|ExecutionSequence`
              (:`then_0`
                (`SceneComponent.K2_SetRelativeRotation` _playerbase (`KismetMathLibrary.RLerp` (`SceneComponent.RelativeRotation` _playerbase) (struct) _alpha) false false))
              (:`then_1`
                (set `SpringArmComponent.TargetArmLength` (`KismetMathLibrary.Lerp` (`SpringArmComponent.TargetArmLength` (`self.SpringArm`)) (`self.MinimumZoom`) _alpha) (`self.SpringArm`)))))))))
  (:`Released`
    (set `self.bIsRotatingCamera` false)
    (set `PlayerController.CurrentMouseCursor` "Default" (`self.PlayerController`))
    (goto _label_2 :!via `Close`)))

(event `InputAction|ResetCamera`
  (params (Key :type "Key Structure"))
  ;[1 1 1] Mouse Middle Button Movement
  (:`Pressed`
    (goto _label_3 :!via `PlayFromStart`)))

(event `Tick_MouseMovement`
  (bind _playercontroller (`self.PlayerController`))
  (bind (_sizex _sizey) (`PlayerController.GetViewportSize` _playercontroller))
  (bind (_locationx _locationy _returnvalue) (`PlayerController.GetMousePosition` _playercontroller))
  ;[1 1 1] Side Scrolling
  (if (and (not (`self.bIsRotatingCamera`)) _returnvalue)
    (`|ExecutionSequence`
      (:`then_0`
        (if (< _locationx (`self.EdgeScrollSensitivity`))
          (`self.AddRight` -1.0)
          (elif (> _locationx (- (`KismetMathLibrary.Conv_IntToDouble` _sizex) (`self.EdgeScrollSensitivity`)))
            (`self.AddRight` 1.0))))
      (:`then_1`
        (if (< _locationy (`self.EdgeScrollSensitivity`))
          (`self.AddForward` 1.0)
          (elif (> _locationy (- (`KismetMathLibrary.Conv_IntToDouble` _sizey) (`self.EdgeScrollSensitivity`)))
            (`self.AddForward` -1.0)))))))

(event `InputAction|IncreaseCameraSpeed`
  (params (Key :type "Key Structure"))
  ;[1 1 1] Mouse Movement
  (:`Pressed`
    (set `self.MovementSpeed` (* (`self.MovementSpeed`) 2.0)))
  (:`Released`
    (set `self.MovementSpeed` (`self.DefaultMovementSpeed`))))

(fn `AddForward`
  (params (axis :type "Float (double-precision)"))
  (`self.K2_AddActorWorldOffset` (* (`SceneComponent.GetForwardVector` (`self.PlayerBase`)) (* (`self.MovementSpeed`) axis))))

(fn `AddRight`
  (params (axis :type "Float (double-precision)"))
  (`self.K2_AddActorWorldOffset` (* (`SceneComponent.GetRightVector` (`self.PlayerBase`)) (* axis (`self.MovementSpeed`)))))

(fn `UserConstructionScript`)